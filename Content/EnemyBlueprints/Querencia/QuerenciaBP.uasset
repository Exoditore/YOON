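; QuerenciaBP is a ranged enemy that chases the player on sight and shoots projectiles at them.
; PawnSensing plays a one-time alert sound and drives AIMoveTo; on arrival it turns to the player and fires on a delay-gated cooldown.
; Damage spawns a splatter, then plays a pain sound and reduces health only with weapon slot 1 or 2 active.
; Death increments the player's kill count, ragdolls the mesh and destroys the actor after a delay.
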(event `self.ReceiveAnyDamage`
  (params (Damage :type "Float (single-precision)") (DamageType :type "DamageType Object Reference") (InstigatedBy :type "Controller Object Reference") (DamageCauser :type "Actor Object Reference"))
  (`GameplayStatics.SpawnEmitterAttached` "/Game/Blueprints/Splatte.Splatte" (`self.Mesh`) "None" (0.0 0.0 1.0) (struct) (0.09 0.09 0.09))
  (if (`/Game/FirstPersonBP/Blueprints/FirstPersonCharacter.WeaponSlot2` (stale `self.ReceiveBeginPlay` _asfirst_person_character))
    (`GameplayStatics.PlaySoundAtLocation` "/Game/song/yt1s_com_-_Doom_1_2_Monster_Sound_effects.yt1s_com_-_Doom_1_2_Monster_Sound_effects" (`SceneComponent.K2_GetComponentLocation` (`self.Audio`)) (struct) 0.3 1.0 0.0 null null null)
    (bind _output_get (set `self.Health` (- (`self.Health`) Damage) :!label _label))
    (if (<= _output_get 0.0)
      (set `self.ded` true)
      (set `/Game/FirstPersonBP/Blueprints/FirstPersonCharacter.KilledEnnemys` (+ (`/Game/FirstPersonBP/Blueprints/FirstPersonCharacter.KilledEnnemys` (stale `self.ReceiveBeginPlay` _asfirst_person_character)) 1.0) (stale `self.ReceiveBeginPlay` _asfirst_person_character))
      (`PrimitiveComponent.SetCollisionEnabled` (`self.CapsuleComponent`) "NoCollision")
      (`PrimitiveComponent.SetCollisionEnabled` (`self.Mesh`) "PhysicsOnly")
      (`PrimitiveComponent.SetSimulatePhysics` (`self.Mesh`) true)
      (`KismetSystemLibrary.Delay` 5.0)
      (`self.K2_DestroyActor`))
    (elif (`/Game/FirstPersonBP/Blueprints/FirstPersonCharacter.WeaponSlot1` (stale `self.ReceiveBeginPlay` _asfirst_person_character))
      (`GameplayStatics.PlaySoundAtLocation` "/Game/song/yt1s_com_-_Doom_1_2_Monster_Sound_effects.yt1s_com_-_Doom_1_2_Monster_Sound_effects" (`SceneComponent.K2_GetComponentLocation` (`self.Audio`)) (struct) 1.0 1.0 0.0 null null null)
      (goto _label))))

(event `self.ReceiveBeginPlay`
  (bind _asfirst_person_character (cast `/Game/FirstPersonBP/Blueprints/FirstPersonCharacter` (`GameplayStatics.GetPlayerCharacter` 0))))

(event `self.PawnSensing.OnSeePawn`
  (params (Pawn :type "Pawn Object Reference"))
  (`self.Sond`)
  (bind _asfirst_person_character (cast `/Game/FirstPersonBP/Blueprints/FirstPersonCharacter` Pawn))
  (`|AIMoveTo` self (0.0 0.0 0.0) _asfirst_person_character 1300.0
    (:`OnSuccess`
      (if (not (`self.ded`))
        (`|ExecutionSequence`
          (:`then_0`
            (`self.K2_SetActorRotation` (`KismetMathLibrary.FindLookAtRotation` (`self.K2_GetActorLocation`) (`self.K2_GetActorLocation` _asfirst_person_character))))
          (:`then_1`
            (if (`self.canAttack`)
              (bind _returnvalue (`|SpawnActorFromClass` "/Game/FirstPersonBP/Blueprints/FirstPersonProjectile.FirstPersonProjectile_C" (`SceneComponent.K2_GetComponentToWorld` (`self.projectile spawn location`)) "Undefined" "OverrideRootScale" null null))
              (`PrimitiveComponent.AddImpulse` (`/Game/FirstPersonBP/Blueprints/FirstPersonProjectile.Sphere` _returnvalue) (* (`SceneComponent.GetForwardVector` (`self.Mesh`)) 200.0) "None" true)
              (set `self.canAttack` false)
              (`KismetSystemLibrary.Delay` 1.5)
              (set `self.canAttack` true))))))))

(event `Sond`
  (`/Engine/EditorBlueprintResources/StandardMacros.DoOnce` false
    (:`Completed`
      (`GameplayStatics.PlaySoundAtLocation` "/Game/Sounds/Enemy/ZombieCue.ZombieCue" (`SceneComponent.K2_GetComponentLocation` (`self.CapsuleComponent`)) (struct) 1.0 1.0 0.0 null null null))))

(fn `UserConstructionScript`)
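; BotonEndLevel is an end-of-level trigger that shows the EndLevel screen when the Action input is held while its Box is overlapped.
; Overlap events, which do not check the overlapping actor, and the input events set two flags that Tick polls.
; When both are true, it disables player character input and shows the mouse cursor, while a DoOnce limits widget creation to one time.
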(event `self.ReceiveBeginPlay`
  (`self.EnableInput` (`GameplayStatics.GetPlayerController` 0)))

(event `self.Box.OnComponentBeginOverlap`
  (params (OverlappedComponent :type "PrimitiveComponent Object Reference") (OtherActor :type "Actor Object Reference") (OtherComp :type "PrimitiveComponent Object Reference") (OtherBodyIndex :type Integer) (bFromSweep :type Boolean) (SweepResult :type "HitResult Structure (by ref)"))
  (set `self.IsOnBox` true))

(event `self.Box.OnComponentEndOverlap`
  (params (OverlappedComponent :type "PrimitiveComponent Object Reference") (OtherActor :type "Actor Object Reference") (OtherComp :type "PrimitiveComponent Object Reference") (OtherBodyIndex :type Integer))
  (set `self.IsOnBox` false))

(event `InputAction|Action` :consume false :overrideparent false
  (params (Key :type "Key Structure"))
  (:`Pressed`
    (set `self.Epressed` true))
  (:`Released`
    (set `self.Epressed` false)))

(event `self.ReceiveTick`
  (params (DeltaSeconds :type "Float (single-precision)"))
  (bind _returnvalue (`GameplayStatics.GetPlayerController` 0))
  (if (and (`self.Epressed`) (`self.IsOnBox`))
    (`self.DisableInput` (`GameplayStatics.GetPlayerCharacter` 0) _returnvalue)
    (set `PlayerController.bShowMouseCursor` true _returnvalue)
    (`/Engine/EditorBlueprintResources/StandardMacros.DoOnce` false
      (:`Completed`
        (bind _returnvalue_2 (`|CreateWidget` "/Game/Hud/EndLevel.EndLevel_C" _returnvalue))
        (bind _output_get (set `self.Player` _returnvalue_2))
        (`UserWidget.AddToViewport` _output_get 0)))))

(fn `UserConstructionScript`)
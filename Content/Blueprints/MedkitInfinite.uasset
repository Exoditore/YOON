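; MedkitInfinite is a respawning health pickup that adds a fixed amount to the first-person player's Vida.
; Any Box overlap triggers it through a DoOnce, applying health to player 0 without checking the overlapping actor or clamping the value.
; It hides the meshes, disables collision, plays a sound and briefly flashes the ItemPickUp widget.
; After a delay it restores visibility and collision and resets the DoOnce.
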(event `self.Box.OnComponentBeginOverlap`
  (params (OverlappedComponent :type "PrimitiveComponent Object Reference") (OtherActor :type "Actor Object Reference") (OtherComp :type "PrimitiveComponent Object Reference") (OtherBodyIndex :type Integer) (bFromSweep :type Boolean) (SweepResult :type "HitResult Structure (by ref)"))
  (`/Engine/EditorBlueprintResources/StandardMacros.DoOnce` false :!label _label
    (:`Completed`
      (bind _output_get (set `self.IsOnbox` true))
      (if _output_get
        (bind _asfirst_person_character (cast `/Game/FirstPersonBP/Blueprints/FirstPersonCharacter` (`GameplayStatics.GetPlayerCharacter` 0)))
        (set `/Game/FirstPersonBP/Blueprints/FirstPersonCharacter.Vida` (+ (`/Game/FirstPersonBP/Blueprints/FirstPersonCharacter.Vida` _asfirst_person_character) 5.0) _asfirst_person_character)
        (`SceneComponent.SetVisibility` (`self.CajaMunicion`) false false)
        (`SceneComponent.SetVisibility` (`self.Plane`) false false)
        (`PrimitiveComponent.SetCollisionEnabled` (`self.Box`) "NoCollision")
        (`PrimitiveComponent.SetCollisionEnabled` (`self.CajaMunicion`) "NoCollision")
        (`GameplayStatics.PlaySound2D` "/Game/Blueprints/Doom_s_Pick_up_Sound.Doom_s_Pick_up_Sound" 2.5 1.0 0.0 null null)
        (bind _returnvalue (`|CreateWidget` "/Game/Hud/ItemPickUp.ItemPickUp_C"))
        (`UserWidget.AddToViewport` _returnvalue 0)
        (`KismetSystemLibrary.Delay` 0.08)
        (`Widget.RemoveFromParent` _returnvalue)
        (`KismetSystemLibrary.Delay` 10.0)
        (`SceneComponent.SetVisibility` (`self.CajaMunicion`) true false)
        (`SceneComponent.SetVisibility` (`self.Plane`) true false)
        (`PrimitiveComponent.SetCollisionEnabled` (`self.CajaMunicion`) "QueryAndPhysics")
        (`PrimitiveComponent.SetCollisionEnabled` (`self.Box`) "QueryAndPhysics")
        (goto _label :!via `Reset`)))))

(fn `UserConstructionScript`)
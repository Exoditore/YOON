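; DoorEnd is a door, likely at a level's end, that opens once the player has killed at least 27 enemies.
; Each tick it checks that the Action input is held, its Box is overlapped and the FirstPersonCharacter's KilledEnnemys count is high enough.
; The Dooranimation timeline then lerps Cube from its relative origin to Cube1's relative location, with a DoOnce playing the Pepe sound at the door.
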(event `self.ReceiveBeginPlay`
  (`self.EnableInput` (`GameplayStatics.GetPlayerController` 0))
  (bind _asfirst_person_character (cast `/Game/FirstPersonBP/Blueprints/FirstPersonCharacter` (`GameplayStatics.GetPlayerCharacter` 0))))

(event `self.Box.OnComponentBeginOverlap`
  (params (OverlappedComponent :type "PrimitiveComponent Object Reference") (OtherActor :type "Actor Object Reference") (OtherComp :type "PrimitiveComponent Object Reference") (OtherBodyIndex :type Integer) (bFromSweep :type Boolean) (SweepResult :type "HitResult Structure (by ref)"))
  (set `self.IsOnBox` true))

(event `self.Box.OnComponentEndOverlap`
  (params (OverlappedComponent :type "PrimitiveComponent Object Reference") (OtherActor :type "Actor Object Reference") (OtherComp :type "PrimitiveComponent Object Reference") (OtherBodyIndex :type Integer))
  (set `self.IsOnBox` false))

(event `InputAction|Action` :consume false :overrideparent false
  (params (Key :type "Key Structure"))
  (:`Pressed`
    (set `self.Epressed` true))
  (:`Released`
    (set `self.Epressed` false)))

(event `self.ReceiveTick`
  (params (DeltaSeconds :type "Float (single-precision)"))
  (if (and (`self.Epressed`) (`self.IsOnBox`) (>= (`/Game/FirstPersonBP/Blueprints/FirstPersonCharacter.KilledEnnemys` (stale `self.ReceiveBeginPlay` _asfirst_person_character)) 27.0))
    (bind (_direction _door) (`Timeline|dooranimation`)
      (:`Update`
        (`SceneComponent.K2_SetRelativeLocation` (`self.Cube`) (`KismetMathLibrary.VLerp` (0.0 0.0 0.0) (`SceneComponent.RelativeLocation` (`self.Cube1`)) _door) false false)
        (`/Engine/EditorBlueprintResources/StandardMacros.DoOnce` false
          (:`Completed`
            (`GameplayStatics.PlaySoundAtLocation` "/Game/song/pepe.pepe" (`SceneComponent.K2_GetComponentLocation` (`self.Cube`)) (struct) 1.0 1.0 0.0 null null null)))))))

(fn `UserConstructionScript`)